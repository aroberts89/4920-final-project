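; Simple enemy character that walks toward the Core and damages it on contact.
; On BeginPlay it uses SimpleMoveToActor to path to the Core, then applies damage on overlap and destroys itself.
; Any damage it receives destroys it immediately, with no health tracking.
; An UpdateWalkSpeed function exposes its movement component's max walk speed to be changed.
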(event `self.ReceiveAnyDamage`
  (params (Damage :type "Float (single-precision)") (DamageType :type "DamageType Object Reference") (InstigatedBy :type "Controller Object Reference") (DamageCauser :type "Actor Object Reference"))
  (`self.K2_DestroyActor`))

(event `self.ReceiveBeginPlay`
  (`AIBlueprintHelperLibrary.SimpleMoveToActor` (`self.GetController`) (`self.Core`)))

(event `self.ReceiveActorBeginOverlap`
  (params (OtherActor :type "Actor Object Reference"))
  (if (== OtherActor (`self.Core`))
    (`GameplayStatics.ApplyDamage` (`self.Core`) 1.0)
    (`self.K2_DestroyActor`)))

(fn `Update Walk Speed`
  (params (NewWalkSpeed :type "Float (double-precision)"))
  (set `CharacterMovementComponent.MaxWalkSpeed` NewWalkSpeed (`self.CharacterMovement`)))

(fn `UserConstructionScript`)