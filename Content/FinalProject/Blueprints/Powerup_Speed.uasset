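; Speed powerup pickup that temporarily boosts the walk speed of the FirstPersonCharacter that touches it.
; On its first overlap only, gated by DoN, it hides itself and multiplies the character movement's MaxWalkSpeed by Multiplier.
; After a Duration delay it divides the speed back and destroys itself.
; An overlap by any other actor still uses up the single trigger and hides the pickup.
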(event `self.ReceiveActorBeginOverlap`
  (params (OtherActor :type "Actor Object Reference"))
  (`/Engine/EditorBlueprintResources/StandardMacros.Do N` 1
    (:`Exit`
      (`self.SetActorHiddenInGame` true)
      (bind _asfirst_person_character (cast `/Game/FirstPersonCPP/Blueprints/FirstPersonCharacter` OtherActor))
      (set `self.PlayerMovement` (`Character.CharacterMovement` _asfirst_person_character))
      (set `CharacterMovementComponent.MaxWalkSpeed` (* (`CharacterMovementComponent.MaxWalkSpeed` (`self.PlayerMovement`)) (`self.Multiplier`)) (`self.PlayerMovement`))
      (`KismetSystemLibrary.Delay` (`self.Duration`))
      (set `CharacterMovementComponent.MaxWalkSpeed` (/ (`CharacterMovementComponent.MaxWalkSpeed` (`self.PlayerMovement`)) (`self.Multiplier`)) (`self.PlayerMovement`))
      (`self.K2_DestroyActor`))))

(fn `UserConstructionScript`)