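; Enemy wave spawner actor that spawns a set number of enemies of a chosen type at its own transform, then removes itself.
; On BeginPlay a DoN loop waits a random delay before each spawn and repeats until the wave count is reached.
; Each enemy gets the spawner's target through an Enemy_Dumb-specific cast, and its destruction is counted; the spawner destroys itself once the whole wave is destroyed.
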(event `self.ReceiveBeginPlay`
  (`/Engine/EditorBlueprintResources/StandardMacros.Do N` (`self.Count`) :!label _label
    (:`Exit`
      (`KismetSystemLibrary.Delay` (`KismetMathLibrary.RandomFloatInRange` 3.0 10.0))
      (bind _returnvalue (`|SpawnActorFromClass` (`self.EnemyType`) (`SceneComponent.K2_GetComponentToWorld` (`self.DefaultSceneRoot`)) "Undefined" "OverrideRootScale" null null))
      (`|ExecutionSequence`
        (:`then_0`
          (bind _asenemy_dumb (cast `/Game/FinalProject/Blueprints/Enemy_Dumb` _returnvalue)) ; TODO - Gonna need a more generic cast here
          (`/Game/FinalProject/Blueprints/Enemy_Dumb.SetTarget` _asenemy_dumb (`self.Target`)))
        (:`then_1`
          (add `self.OnDestroyed` _returnvalue (delegate `WaveMemberDestroyed`)))
        (:`then_2`
          (goto _label))))))

(event `WaveMemberDestroyed` :!signature `self.OnDestroyed`
  (params (DestroyedActor :type "Actor Object Reference"))
  (bind _result (`/Engine/EditorBlueprintResources/StandardMacros.IncrementInt` (`self.Destroyed`))
    (:`  `
      (if (== _result (`self.Count`))
        (`self.K2_DestroyActor`)))))

(fn `UserConstructionScript`)